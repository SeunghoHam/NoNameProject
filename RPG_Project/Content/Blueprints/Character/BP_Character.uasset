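; Player character Blueprint for an RPG that handles camera-relative movement, look input and detection of interactable actors.
; Movement follows control yaw only, and BeginPlay caches the HUD from RPGGameMode.
; InteractCheck, run on Interact press and every MoveForward axis event, sphere-traces from the actor along the camera's forward direction with debug drawing.
; Initial-overlap hits implementing InteractInterface are stored and their names printed, with no interface call.
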(event EventBeginPlay
  (bind _asrpggame_mode (Utilities|Casting|CastToRPGGameMode (Game|GetGameMode)))
  (Variables|Default|SetPlayersHUD (Variables|/Game/Blueprints/GameMode/RPGGameMode.RPGGameMode_C|GetHeadsUpDisplay _asrpggame_mode)))

(event Input|ActionEvents|InputActionInteract
  (params (Key :type Key%20Structure :default "None"))
  (:Pressed
    (CallFunction|InteractCheck)))

(event Input|AxisEvents|InputAxisLookUp
  (params (AxisValue :type Float%20%28single-precision%29))
  ;[1 1 1] About Move&Look
  (Pawn|Input|AddControllerPitchInput AxisValue))

(event Input|AxisEvents|InputAxisTurnRate
  (params (AxisValue :type Float%20%28single-precision%29))
  ;[1 1 1] About Move&Look
  (Pawn|Input|AddControllerYawInput (* AxisValue (Variables|Default|GetBaseTurnRate) (Utilities|Time|GetWorldDeltaSeconds))))

(event Input|AxisEvents|InputAxisTurn
  (params (AxisValue :type Float%20%28single-precision%29))
  ;[1 1 1] About Move&Look
  (Pawn|Input|AddControllerYawInput AxisValue))

(event Input|AxisEvents|InputAxisLookUpRate
  (params (AxisValue :type Float%20%28single-precision%29))
  ;[1 1 1] About Move&Look
  (Pawn|Input|AddControllerPitchInput (* AxisValue (Variables|Default|GetBaseLookUpRate) (Utilities|Time|GetWorldDeltaSeconds))))

(event Input|AxisEvents|InputAxisMoveForward
  (params (AxisValue :type Float%20%28single-precision%29))
  ;[1 1 1] About Move&Look
  (Pawn|Input|AddMovementInput (Math|Vector|GetForwardVector (Math|Rotator|MakeRotator 0.0 0.0 (.Yaw (Math|Rotator|BreakRotator (Pawn|GetControlRotation :!class /Script/Engine.Pawn))))) AxisValue false)
  (CallFunction|InteractCheck))

(event Input|AxisEvents|InputAxisMoveRight
  (params (AxisValue :type Float%20%28single-precision%29))
  ;[1 1 1] About Move&Look
  (Pawn|Input|AddMovementInput (Math|Vector|GetRightVector (Math|Rotator|MakeRotator 0.0 0.0 (.Yaw (Math|Rotator|BreakRotator (Pawn|GetControlRotation :!class /Script/Engine.Pawn))))) AxisValue false))

(fn ConstructionScript)

(fn InteractCheck
  (bind _returnvalue (Transformation|GetActorLocation))
  (bind _outhit (Collision|SphereTraceByChannel _returnvalue (+ _returnvalue (* (Math|Vector|GetForwardVector (Transformation|GetWorldRotation (Variables|Default|GetCamera))) 2e+02)) 5e+01 "TraceTypeQuery2" false 0 "ForOneFrame"))
  (if (.binitialoverlap _outhit)
    (if (Utilities|DoesObjectImplementInterface (.hitactor _outhit) "/Game/Blueprints/Interface/InteractInterface.InteractInterface_C")
      ;[1 1 1] LocalVarient
      (bind _output_get (LocalVariables|SetInteractActor (.hitactor _outhit)))
      (Development|PrintString (Utilities|GetDisplayName _output_get)))))